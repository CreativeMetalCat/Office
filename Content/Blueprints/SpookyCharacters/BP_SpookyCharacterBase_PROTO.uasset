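; Prototype base Blueprint for a spooky zombie that attacks the table player unless held back with light.
; After a spawn animation, an attack starts a shadow timer that ends in a scream and jumpscare.
; Light changes pause and resume that timer against a shine timer, which cancels the attack when it expires.
; Cancellation plays the despawn, waits out a cooldown, then queues a new action at a random allowed location on the player.
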(event Custom|CooldownAndAttack
  (bind _player (Variables|Default|GetPlayer))
  ;[1 1 1] Attack again
  (Audio|PlaySound2D "/Game/Sounds/HorrorSoundPack/Audio/Wav/bam.bam" 0.2 1.0 0.0 0 0)
  (Utilities|Time|ClearandInvalidateTimerbyHandle (Variables|LightTimers|GetShineTimer))
  (Utilities|Time|ClearandInvalidateTimerbyHandle (Variables|LightTimers|GetNoLightTimer))
  (Components|Animation|PlayAnimation (Variables|Default|GetSK_Zombie_1) "/Game/Polygonmaker/Animations/Undead/Anim_Zombie_despawn.Anim_Zombie_despawn" false)
  (Utilities|FlowControl|Delay (Variables|Default|GetCooldown))
  (Utilities|IsValid _player
    (:Is%20Valid
      (bind _structout (Utilities|Struct|SetmembersinS_SpookyCharacterAction (Variables|AIAction|GetAction) (.OutItem (Utilities|Array|Random (Variables|Locations|GetAllowedLocations)))))
      (Default|AddAction _player _structout))))

(event Custom|DoPreparation
  (Components|Animation|PlayAnimation (Variables|Default|GetSK_Zombie_1) "/Game/Polygonmaker/Animations/Undead/Anim_Zombie_spawn.Anim_Zombie_spawn" false)
  (Utilities|FlowControl|Delay 4.0)
  (Variables|Default|SetReady true)
  (Components|Animation|PlayAnimation (Variables|Default|GetSK_Zombie_1) "/Game/Polygonmaker/Animations/Undead/Anim_Zombie_idle.Anim_Zombie_idle" false))

(event EventBeginPlay
  ;[1 1 1] Generate Sturct
  (bind _structout (Utilities|Struct|SetmembersinS_SpookyCharacterAction (Variables|AIAction|GetAction) self))
  (Variables|AIAction|SetAction _structout)
  (bind _outactors (Actor|GetAllActorsOfClass "/Game/Blueprints/Player/BP_Player_Table_PROTO.BP_Player_Table_PROTO_C"))
  (Variables|Default|SetPlayer (Utilities|Array|Get(acopy) _outactors))
  (EventDispatchers|BindEventtoAttackCanceled (delegate Custom|CooldownAndAttack)))

(fn ConstructionScript)

(fn PerfromAttack
  (bind _returnvalue (Utilities|Time|SetTimerbyFunctionName self "OnStayedInShadowForEnoughTime" (Variables|Default|GetWaitTimeBeforeAttack)))
  (Variables|LightTimers|SetNoLightTimer _returnvalue)
  (Audio|PlaySoundatLocation "/Game/Sounds/Horror/breath2_Cue.breath2_Cue" (Transformation|GetActorLocation) "0, 0, 0" 1.0 1.0 0.0 0 0 0)
  (Variables|Default|SetReady false))

(fn OnStayedinShadowforEnoughTime
  (Audio|PlaySound2D "/Game/Sounds/HorrorSoundPack/Audio/Wav/screamzombie.screamzombie" 1.0 1.0 0.0 0 0)
  (CallFunction|DoJumpscare))

(fn ReacttoLight
  (params (LightIsTurnedOff :type Boolean))
  (bind _nolighttimer (Variables|LightTimers|GetNoLightTimer))
  (if (Utilities|Time|IsValidTimerHandle (Variables|LightTimers|GetNoLightTimer))
    ;[1 1 1] React to light on
    (if (not LightIsTurnedOff)
      (Utilities|Time|PauseTimerbyHandle _nolighttimer)
      (if (not (Utilities|Time|IsValidTimerHandle (Variables|LightTimers|GetShineTimer)))
        (bind _returnvalue (Utilities|Time|SetTimerbyFunctionName self "OnLightShinedForEnoughTime" (Variables|Default|GetShineAtTime)))
        (Variables|LightTimers|SetShineTimer _returnvalue)
        (else
          (Utilities|Time|UnpauseTimerbyHandle (Variables|LightTimers|GetShineTimer))))
      (else
        ;[1 1 1] react to lights off
        (Utilities|Time|UnpauseTimerbyHandle _nolighttimer)
        (if (Utilities|Time|IsValidTimerHandle (Variables|LightTimers|GetShineTimer))
          (Utilities|Time|PauseTimerbyHandle (Variables|LightTimers|GetShineTimer)))))))

(fn OnLightShinedforEnoughTime
  (Default|CallAttackCanceled)
  (Transformation|SetRelativeLocation (Variables|Default|GetSK_Zombie_1) "0, 0, 0" false false))

(fn Prepare
  (params (SpawnPoint :type BP%20Spawn%20Point%20Object%20Reference))
  (CallFunction|DoPreparation))

(fn DoJumpscare
  (Default|MovetoJumpscarePosition (Variables|Default|GetPlayer) self)
  (Components|Animation|PlayAnimation (Variables|Default|GetSK_Zombie_1) "/Game/Polygonmaker/Animations/Undead/Anim_Zombie_taunt.Anim_Zombie_taunt" false)
  (Utilities|Time|SetTimerbyEvent (EventDispatchers|CreateEvent (Variables|Default|GetPlayer) :!event DoEndScreen) 2.0))