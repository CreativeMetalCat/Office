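; BP_Player_Walk is the walking player pawn, handling the Interact input and the switch to a seated table pawn for PC use.
; It caches its PlayerController on BeginPlay.
; If Interact finds an overlapping BP_Player_Table_PROTO, it blends the camera to the first one, possesses it after the blend and calls BePossesed.
; Otherwise it sends InteractMessage, passing itself, to every actor overlapping the capsule.
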(event EventBeginPlay
  ;[1 1 1] Record value of controller
  (bind _asplayer_controller (Utilities|Casting|CastToPlayerController (Pawn|GetController)))
  (Variables|Default|SetPlayer%20Controller _asplayer_controller))

(event Input|ActionEvents|InputActionInteract
  (params (Key :type Key%20Structure :default "None"))
  (bind _capsulecomponent (Variables|Default|GetCapsuleComponent))
  (bind _player_controller (Variables|Default|GetPlayer%20Controller))
  (bind _overlappingactors (Collision|GetOverlappingActors _capsulecomponent "/Game/Blueprints/Player/BP_Player_Table_PROTO.BP_Player_Table_PROTO_C" :!class /Script/Engine.PrimitiveComponent))
  (bind _output (Utilities|Array|Get(acopy) _overlappingactors))
  (bind _asbp_player_table_proto (Utilities|Casting|CastToBP_Player_Table_PROTO _output))
  ;[1 1 1] Sit down to use pc
  (:Pressed
    (if (> (Utilities|Array|Length _overlappingactors) 0)
      (Game|Player|SetViewTargetwithBlend (Variables|Default|GetPlayer%20Controller) _output 0.5 "VTBlend_Linear" 0.0 false)
      (Utilities|FlowControl|Delay 0.5)
      (Pawn|Possess _player_controller _asbp_player_table_proto)
      (Default|BePossesed _asbp_player_table_proto _player_controller)
      (else
        ;[1 1 1] If no table player found - just interact with everything
        (for _array_element (Collision|GetOverlappingActors _capsulecomponent "/Script/Engine.Actor" :!class /Script/Engine.PrimitiveComponent)
          (Class|InteractionInterface|Interact(Message) _array_element self))))))

(fn ConstructionScript)