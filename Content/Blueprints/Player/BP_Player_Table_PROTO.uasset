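; Prototype player seated at a table that tracks work progress while possessed, adds a HUD, and manages AI character attacks.
; Held look inputs blend to directional camera actors through ChangeCamera's half-second lock; Tick restores the default view, and flashlight input drives the current BP_Camera.
; AddAction attacks immediately when the action list is empty, otherwise queues the character at WaitLocation; cancellation removes the last entry and triggers the next after a cooldown.
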(event Custom|BePossesed
  (params (Player%20Controller :type Player%20Controller%20Object%20Reference))
  ;[1 1 1] Be possesed
  (Variables|Default|SetCurrentlyControlledByPlayer true)
  (Variables|Default|SetPlayer%20Controller Player%20Controller)
  ;[1 1 1] Add hud
  (bind _returnvalue (UserInterface|CreateWidget "/Game/Blueprints/UMG_Table_Hud.UMG_Table_Hud_C" (Variables|Default|GetPlayer%20Controller) self))
  (UserInterface|Viewport|AddtoViewport _returnvalue 0)
  (Variables|Default|SetHUD _returnvalue)
  (Default|CallOnPossessed))

(event Custom|CallPerformAttack
  (params (Character :type BP%20Spooky%20Character%20Base%20PROTO%20Object%20Reference) (LocationId :type Integer))
  ;[1 1 1] Make Ai perform attack
  (EventDispatchers|BindEventtoAttackCanceled Character (delegate Custom|OnAttackCanceled))
  (Transformation|SetActorLocation Character (Transformation|GetActorLocation (Utilities|Array|Get(acopy) (Variables|Locations|GetLocations) LocationId)) false false)
  (Default|PerfromAttack Character))

(event Custom|OnAttackCanceled
  (bind _actions (Variables|Enemies|GetActions))
  (bind _actions_2 (Variables|Enemies|GetActions))
  (bind _returnvalue (Utilities|Array|Length _actions_2))
  ;[1 1 1] If attack was canlced we still have to remove it
  (Utilities|Array|RemoveIndex _actions (- (Utilities|Array|Length _actions) 1))
  ;[1 1 1] Start next action
  (if (> _returnvalue 0)
    (Utilities|FlowControl|Delay (Variables|Default|GetCooldownTime))
    (CallFunction|CallPerformAttack (.Character (Utilities|Struct|BreakS_SpookyCharacterAction (Utilities|Array|Get(acopy) _actions_2 (- _returnvalue 1)))))))

(event EventBeginPlay)

(event EventTick
  (params (DeltaSeconds :type Float%20%28single-precision%29))
  (if (Variables|Default|GetCurrentlyControlledByPlayer)
    ;[1 1 1] Update progress
    (bind _output_get (Variables|Work|SetWorkTime (+ DeltaSeconds (Variables|Work|GetWorkTime))))
    (Variables|Work|SetWorkProgress (/ _output_get (Variables|Work|GetNeededWorkTime)))
    ;[1 1 1] Switch back to default camera
    (if (and (not (Variables|Default|GetResetToDefaultCamera)) (not (Variables|Default|GetCameraUsed)))
      (Utilities|ChangeCamera self 0.25
        (:Started
          (Variables|Default|SetCameraUsed false)
          (Variables|Default|SetResetToDefaultCamera true))))))

(event Input|ActionEvents|InputActionTable_LookUp
  (params (Key :type Key%20Structure :default "None"))
  ;[1 1 1] Turn player's head
  (:Pressed
    (Utilities|ChangeCamera (Variables|Cameras|GetUpCameraActor) 0.2
      (:Started
        (Variables|Default|SetCameraUsed true)
        (Variables|Default|SetResetToDefaultCamera false))))
  (:Released
    (Variables|Default|SetCameraUsed false)))

(event Input|ActionEvents|InputActionTable_LookBehind
  (params (Key :type Key%20Structure :default "None"))
  ;[1 1 1] Turn player's head
  (:Pressed
    (Utilities|ChangeCamera (Variables|Cameras|GetBackCameraActor) 0.1
      (:Started
        (Variables|Default|SetCameraUsed true)
        (Variables|Default|SetResetToDefaultCamera false))))
  (:Released
    (Variables|Default|SetCameraUsed false)))

(event Input|ActionEvents|InputActionTable_LookRight
  (params (Key :type Key%20Structure :default "None"))
  ;[1 1 1] Turn player's head
  (:Pressed
    (Utilities|ChangeCamera (Variables|Cameras|GetRightCameraActor) 0.5
      (:Started
        (Variables|Default|SetCameraUsed true)
        (Variables|Default|SetResetToDefaultCamera false))))
  (:Released
    (Variables|Default|SetCameraUsed false)))

(event Input|ActionEvents|InputActionTable_LookLeft
  (params (Key :type Key%20Structure :default "None"))
  ;[1 1 1] Turn player's head
  (:Pressed
    (Utilities|ChangeCamera (Variables|Cameras|GetLeftCameraActor) 0.5
      (:Started
        (Variables|Default|SetCameraUsed true)
        (Variables|Default|SetResetToDefaultCamera false))))
  (:Released
    (Variables|Default|SetCameraUsed false)))

(event Input|ActionEvents|InputActionTable_Flashlight
  (params (Key :type Key%20Structure :default "None"))
  (bind _currentcamera (Variables|Default|GetCurrentCamera))
  ;[1 1 1] Flashlight
  (:Pressed
    (Utilities|IsValid _currentcamera
      (:Is%20Valid
        (Default|ActivateFlashlight _currentcamera))))
  (:Released
    (Utilities|IsValid _currentcamera
      (:Is%20Valid
        (Default|DeactivateFlashlight _currentcamera)))))

(fn ConstructionScript)

(fn AddAction
  (params (Action :type S%20Spooky%20Character%20Action%20Structure))
  (bind (_character _lenght _locationid) (Utilities|Struct|BreakS_SpookyCharacterAction Action))
  (bind _actions (Variables|Enemies|GetActions))
  (if (!= (Utilities|Array|Length _actions) 0)
    (Utilities|Array|Add _actions Action)
    (Transformation|SetActorLocation _character (Transformation|GetActorLocation (Variables|Locations|GetWaitLocation)) false false)
    (else
      (CallFunction|CallPerformAttack _character _locationid))))