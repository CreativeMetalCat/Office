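; Prototype player that looks up, behind, left or right by blending the view to separate camera actors while a Table look input is held.
; On release, Tick blends back to the player's own view.
; The ChangeCamera macro performs each blend, caches the target if it is a BP_Camera, and locks further switches for a short delay.
; Flashlight input switches the light on that cached camera while held.
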(event EventBeginPlay
  (bind _asplayer_controller (Utilities|Casting|CastToPlayerController (Pawn|GetController)))
  (Variables|Default|SetPlayer%20Controller _asplayer_controller))

(event Collision|EventActorBeginOverlap
  (params (OtherActor :type Actor%20Object%20Reference)))

(event EventTick
  (params (DeltaSeconds :type Float%20%28single-precision%29))
  (if (and (not (Variables|Default|GetResetToDefaultCamera)) (not (Variables|Default|GetCameraUsed)))
    (Utilities|ChangeCamera self 0.5
      (:Started
        (Variables|Default|SetCameraUsed false)
        (Variables|Default|SetResetToDefaultCamera true)))))

(event Input|ActionEvents|InputActionTable_LookUp
  (params (Key :type Key%20Structure :default "None"))
  (:Pressed
    (Utilities|ChangeCamera (Variables|Cameras|GetUpCameraActor) 0.2
      (:Started
        (Variables|Default|SetCameraUsed true)
        (Variables|Default|SetResetToDefaultCamera false))))
  (:Released
    (Variables|Default|SetCameraUsed false)))

(event Input|ActionEvents|InputActionTable_LookBehind
  (params (Key :type Key%20Structure :default "None"))
  (:Pressed
    (Utilities|ChangeCamera (Variables|Cameras|GetBackCameraActor) 0.1
      (:Started
        (Variables|Default|SetCameraUsed true)
        (Variables|Default|SetResetToDefaultCamera false))))
  (:Released
    (Variables|Default|SetCameraUsed false)))

(event Input|ActionEvents|InputActionTable_LookRight
  (params (Key :type Key%20Structure :default "None"))
  (:Pressed
    (Utilities|ChangeCamera (Variables|Cameras|GetRightCameraActor) 0.5
      (:Started
        (Variables|Default|SetCameraUsed true)
        (Variables|Default|SetResetToDefaultCamera false))))
  (:Released
    (Variables|Default|SetCameraUsed false)))

(event Input|ActionEvents|InputActionTable_LookLeft
  (params (Key :type Key%20Structure :default "None"))
  (:Pressed
    (Utilities|ChangeCamera (Variables|Cameras|GetLeftCameraActor) 0.5
      (:Started
        (Variables|Default|SetCameraUsed true)
        (Variables|Default|SetResetToDefaultCamera false))))
  (:Released
    (Variables|Default|SetCameraUsed false)))

(event Input|ActionEvents|InputActionTable_Flashlight
  (params (Key :type Key%20Structure :default "None"))
  (bind _currentcamera (Variables|Default|GetCurrentCamera))
  ;[1 1 1] Flashlight
  (:Pressed
    (Utilities|IsValid _currentcamera
      (:Is%20Valid
        (Default|ActivateFlashlight _currentcamera))))
  (:Released
    (Utilities|IsValid _currentcamera
      (:Is%20Valid
        (Default|DeactivateFlashlight _currentcamera)))))

(fn ConstructionScript)